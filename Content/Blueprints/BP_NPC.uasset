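; BP_NPC is an AI-controlled pawn that idles, patrols or runs from the player according to its AIState.
; BeginPlay starts Idle (an empty placeholder) or a patrol that loops through PatrolPoints with AI MoveTo, advancing only on success.
; Tick handles Idle and fleeing, which passes the player pawn to MoveAwayFromPawn on NPCAIController.
; Tick has no Patrol case, so patrolling starts only from BeginPlay.
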(event Custom|RunFromPlayer
  ;[1 1 1] AI Run From Player
  (bind _asnpcaicontroller (Utilities|Casting|CastToNPCAIController (AI|GetAIController self)))
  (bind _returnvalue (Class|NPCAIController|GetPlayerPawn _asnpcaicontroller))
  (Class|NPCAIController|MoveAwayfromPawn _asnpcaicontroller _returnvalue))

(event Custom|Idle)

(event Custom|PatrolToPoint
  ;[1 1 1] AI Patrol To Point
  (AI|AIMoveTo self "0, 0, 0" (Utilities|Array|Get(acopy) (Variables|Default|GetPatrolPoints) (Variables|Default|GetPatrolPointIndex)) 5.0 false
    (:OnSuccess
      (if (>= (Variables|Default|GetPatrolPointIndex) (- (Utilities|Array|Length (Variables|Default|GetPatrolPoints)) 1))
        (Variables|Default|SetPatrolPointIndex 0)
        (else
          (Math|Integer|IncrementInt (Variables|Default|GetPatrolPointIndex)
            (:%20%20
              _))))
      (CallFunction|PatroltoPoint))))

(event EventBeginPlay
  (switch Utilities|FlowControl|Switch|SwitchonEAIState (Variables|Default|GetAIState)
    (:NewEnumerator0
      (CallFunction|Idle))
    (:NewEnumerator3
      (CallFunction|PatroltoPoint))))

(event EventTick
  (params (DeltaSeconds :type Float%20%28single-precision%29))
  (switch Utilities|FlowControl|Switch|SwitchonEAIState (Variables|Default|GetAIState)
    (:NewEnumerator0
      (CallFunction|Idle))
    (:NewEnumerator1
      (CallFunction|RunfromPlayer))))

(fn ConstructionScript
  (|CallParentFunction))